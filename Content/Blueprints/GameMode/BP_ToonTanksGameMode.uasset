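; Game mode Blueprint for Toon Tanks that handles start-of-game and game-over UI.
; StartGame briefly delays, shows the main menu with UI-only input and cursor, then pauses.
; A Delay after the pause holds back the start-game widget until play resumes.
; GameOver shows an end-game widget with win or lose text, enables game-and-UI input with cursor, and leaves the game unpaused.
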(event `self.StartGame`
  (bind _returnvalue (`GameplayStatics.GetPlayerController` 0))
  (`KismetSystemLibrary.Delay` 0.05)
  (bind _returnvalue_2 (`|CreateWidget` "/Game/Blueprints/Widgets/WB_MainMenu.WB_MainMenu_C"))
  (`UserWidget.AddToViewport` _returnvalue_2 0)
  (`WidgetBlueprintLibrary.SetInputMode_UIOnlyEx` _returnvalue null)
  (set `PlayerController.bShowMouseCursor` true _returnvalue)
  (`GameplayStatics.SetGamePaused` true)
  (`KismetSystemLibrary.Delay` 0.1)
  (bind _returnvalue_3 (`|CreateWidget` "/Game/Blueprints/Widgets/WB_StartGameWidget.WB_StartGameWidget_C"))
  (`UserWidget.AddToViewport` _returnvalue_3 0))

(event `self.GameOver`
  (params (bWonGame :type Boolean))
  (bind _returnvalue (`GameplayStatics.GetPlayerController` 0))
  (bind _returnvalue_2 (`|CreateWidget` "/Game/Blueprints/Widgets/WB_EndGameWidget.WB_EndGameWidget_C" _returnvalue))
  (`UserWidget.AddToViewport` _returnvalue_2 0)
  (set `TextBlock.Text` (select `bool` bWonGame :`false` "You Lost!" :`true` "You Won!" :!type "Text") (`/Game/Blueprints/Widgets/WB_EndGameWidget.DisplayText` _returnvalue_2))
  (`WidgetBlueprintLibrary.SetInputMode_GameAndUIEx` _returnvalue null)
  (set `PlayerController.bShowMouseCursor` true (`GameplayStatics.GetPlayerController` 0))
  (`GameplayStatics.SetGamePaused` false))

(fn `UserConstructionScript`)