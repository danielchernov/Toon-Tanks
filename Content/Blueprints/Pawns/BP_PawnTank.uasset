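; Tank pawn Blueprint whose only graph logic is an Escape-key toggle for the pause menu.
; Opening creates a WB_PauseMenu widget, adds it to the viewport, focuses it in Game and UI input mode, shows the cursor and pauses the game.
; Closing removes the widget, unpauses, restores game-only input and hides the cursor, with IsPauseMenuOpen tracking the state.
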(event `Key|Escape`
  (params (Key :type "Key Structure"))
  (bind _returnvalue (`GameplayStatics.GetPlayerController` 0))
  (:`Pressed`
    (if (not (`self.isPauseMenuOpen`))
      (set `self.isPauseMenuOpen` true)
      (bind _returnvalue_2 (`|GenericCreateObject` _returnvalue "/Game/Blueprints/Widgets/WB_PauseMenu.WB_PauseMenu_C"))
      (bind _output_get (set `self.PauseMenuWidget` _returnvalue_2))
      (`UserWidget.AddToViewport` _output_get 0)
      (`WidgetBlueprintLibrary.SetInputMode_GameAndUIEx` _returnvalue (`self.PauseMenuWidget`))
      (set `PlayerController.bShowMouseCursor` true (`GameplayStatics.GetPlayerController` 0))
      (`GameplayStatics.SetGamePaused` true)
      (else
        (set `self.isPauseMenuOpen` false)
        (`Widget.RemoveFromParent` (`self.PauseMenuWidget`))
        (`GameplayStatics.SetGamePaused` false)
        (`WidgetBlueprintLibrary.SetInputMode_GameOnly` _returnvalue)
        (set `PlayerController.bShowMouseCursor` false (`GameplayStatics.GetPlayerController` 0))))))

(fn `UserConstructionScript`)